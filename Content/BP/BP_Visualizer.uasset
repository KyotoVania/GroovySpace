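; Music visualizer actor that plays a ConstantQNRT asset's sound and animates a row of BP_SoundCube actors spawned at BeginPlay.
; Each playback-percent callback converts progress to song time and reads baked Constant-Q band strengths to scale the matching cubes.
; Bands above Treshold times Difficulty emit pooled BP_SoundSpheres through BP_PoolManager, gated by a per-cube cooldown.
; An input action toggles pause; the runtime audio import code is unreachable.
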(event Custom|OnPlaybackChange
  (params (PlayingSoundWave :type Sound%20Wave%20Object%20Reference) (PlaybackPercent :type Float%20%28single-precision%29))
  ;[0.15 0.15 0.15 0.5] SetPlayBackLink
  (CallFunction|SynthesiaScale (Variables|Default|GetMusicDuration) PlaybackPercent (Variables|Default|GetSound%20Cube%20Ref)))

(event Custom|OnResult_Event
  (params (Importer :type Runtime%20Audio%20Importer%20Library%20Object%20Reference) (ImportedSoundWave :type Imported%20Sound%20Wave%20Object%20Reference) (Status :type ERuntimeImportStatus%20Enum :default "SuccessfulImport"))
  (Variables|Default|SetImporter 0)
  (if (not (Utilities|Enum|Equal(Enum) Status "SuccessfulImport"))
    (Development|PrintString "failed")))

(event Input|EnhancedActionEvents|EnhancedInputActionIA_PauseAction
  (params (ActionValue :type Boolean) (ElapsedSeconds :type Float%20%28double-precision%29) (TriggeredSeconds :type Float%20%28double-precision%29) (InputAction :type Input%20Action%20Object%20Reference :default "/Game/Player/inputs/Actions/IA_PauseAction.IA_PauseAction"))
  (bind _audio (Variables|Default|GetAudio))
  ;[0.15 0.15 0.15 0.5] Pause/Start
  (:Completed
    (Development|PrintString "Hello")
    (if (Audio|Components|Audio|IsPlaying (Variables|Default|GetAudio))
      (bind _isa (Utilities|FlowControl|FlipFlop)
        (:A
          _)
        (:B
          _))
      (Class|AudioComponent|SetPaused _audio _isa)
      (else
        (Audio|Components|Audio|Play _audio 0.0)))))

(event Input|EnhancedActionEvents|EnhancedInputActionIA_SwitchAction
  (params (ActionValue :type Boolean) (ElapsedSeconds :type Float%20%28double-precision%29) (TriggeredSeconds :type Float%20%28double-precision%29) (InputAction :type Input%20Action%20Object%20Reference :default "/Game/Player/inputs/Actions/IA_SwitchAction.IA_SwitchAction")))

(event EventBeginPlay
  (bind _audio (Variables|Default|GetAudio))
  (bind _constantqnrt (Variables|Default|GetConstantQNRT))
  (bind _sound (Variables|/Script/AudioAnalyzer.AudioAnalyzerNRT|GetSound _constantqnrt))
  (Utilities|FlowControl|Sequence
    (:then_0
      ;[0.15 0.15 0.15 0.5] Input
      (Input|EnableInput (Game|GetPlayerController 0))
      (bind _returnvalue (Actor|GetActorOfClass "/Game/BP/BP_SongSelector.BP_SongSelector_C"))
      (Variables|Default|SetSongSelector _returnvalue))
    (:then_1
      ;[0.15 0.15 0.15 0.5] Init
      (Audio|Components|Audio|SetSound (Variables|Default|GetAudio) _sound)
      (Variables|Default|SetMusicDuration (Variables|/Script/Engine.SoundBase|GetDuration _sound))
      (bind _returnvalue_2 (Actor|GetActorOfClass "/Game/BP/BP_PoolManager.BP_PoolManager_C"))
      (Variables|Default|SetPoolManager _returnvalue_2))
    (:then_2
      ;[0.15 0.15 0.15 0.5] Spawn Cube
      (bind _soundcuberef (CallFunction|SpawnAudio (Variables|Default|GetNumber%20Of%20Cube) (Variables|Default|GetSpacing%20Between)))
      (Variables|Default|SetSound%20Cube%20Ref _soundcuberef))
    (:then_3
      ;[0.15 0.15 0.15 0.5] SetPlayBackLink
      (EventDispatchers|BindEventtoOnAudioPlaybackPercent (Variables|Default|GetAudio) (delegate Custom|OnPlaybackChange)))
    (:then_4
      ;[0.15 0.15 0.15 0.5] Pause/Start
      (Development|PrintString "Hello")
      (if (Audio|Components|Audio|IsPlaying (Variables|Default|GetAudio))
        (bind _isa (Utilities|FlowControl|FlipFlop)
          (:A
            _)
          (:B
            _))
        (Class|AudioComponent|SetPaused _audio _isa)
        (else
          (Audio|Components|Audio|Play _audio 0.0))))))

(event Collision|EventActorBeginOverlap
  (params (OtherActor :type Actor%20Object%20Reference)))

(event EventTick
  (params (DeltaSeconds :type Float%20%28single-precision%29)))

(fn ConstructionScript)

(fn SpawnAudio
  (params (NumberOfCube :type Integer) (SpacingBetween :type Float%20%28double-precision%29))
  (bind _defaultsceneroot (Variables|Default|GetDefaultSceneRoot))
  (bind _returnvalue (Transformation|GetWorldLocation _defaultsceneroot))
  ;[0.15 0.15 0.15 0.5] SpawnCube
  (for _index (range 1 NumberOfCube)
    (Game|SpawnActorfromClass "/Game/ItemBP/BP_SoundCube.BP_SoundCube_C" (Math|Transform|MakeTransform (Math|Vector|MakeVector (.x _returnvalue) (+ (.y _returnvalue) (* _index SpacingBetween)) (.z _returnvalue)) "0, 0, 0" "0.250000,0.250000,0.250000") "Undefined" "MultiplyWithRoot" 0 0))
  ;[0.15 0.496 0.15 0.5] Return all the spawned Cube as array
  (bind _outactors (Actor|GetAllActorsOfClass "/Game/ItemBP/BP_SoundCube.BP_SoundCube_C"))
  (return _outactors))

(fn SynthesiaScale
  (params (MusicDuration :type Float%20%28double-precision%29) (PercentagePlayed :type Float%20%28double-precision%29) (SoundCube :type Array%20of%20BP%20Sound%20Cube%20Object%20References))
  (Utilities|FlowControl|Sequence
    (:then_0
      ;[0.15 0.15 0.15 0.5] Get Space In track
      (Variables|Default|SetSpaceInMusic (* MusicDuration PercentagePlayed)))
    (:then_1
      ;[0.15 0.15 0.15 0.5] Get Result for Frame
      (Variables|Default|SetFrequency%20Band%20Strenght (Class|ConstantQNRT|GetNormalizedChannelConstantQatTime (Variables|Default|GetConstantQNRT) (Variables|Default|GetSpaceInMusic))))
    (:then_2
      ;[0.15 0.15 0.15 0.5] Apply scaling
      (for (_array_element _array_index) (Variables|Default|GetFrequency%20Band%20Strenght)
        (if (> _array_element (* (Variables|Default|GetTreshold) (Variables|Default|Getdifficulty)))
          (if (<= (Variables|/Game/ItemBP/BP_SoundCube.BP_SoundCube_C|GetSpawnCooldown (Utilities|Array|Get(acopy) SoundCube _array_index)) 0.0)
            (Variables|/Game/ItemBP/BP_SoundCube.BP_SoundCube_C|SetSpawnCooldown (Utilities|Array|Get(acopy) SoundCube _array_index) 0.3)
            (bind _newparam (Default|GetPooledObject (Variables|Default|GetPoolManager) (Math|Transform|MakeTransform (.location (Transformation|GetWorldTransform (Variables|/Game/ItemBP/BP_SoundCube.BP_SoundCube_C|GetCube (Utilities|Array|Get(acopy) SoundCube _array_index)))) (.rotation (Transformation|GetWorldTransform (Variables|/Game/ItemBP/BP_SoundCube.BP_SoundCube_C|GetCube (Utilities|Array|Get(acopy) SoundCube _array_index)))))))
            (bind _asbp_sound_sphere (Utilities|Casting|CastToBP_SoundSphere _newparam)
              (:then
                (Variables|/Game/ItemBP/BP_SoundSphere.BP_SoundSphere_C|Setspeed _asbp_sound_sphere (* (- _array_element 0.5) 2e+03))
                (Variables|/Game/ItemBP/BP_SoundSphere.BP_SoundSphere_C|SetFusionTimer%20 _asbp_sound_sphere 1.0)
                (Variables|/Game/ItemBP/BP_SoundSphere.BP_SoundSphere_C|SetIsMerging _asbp_sound_sphere false)
                (Variables|/Game/ItemBP/BP_SoundSphere.BP_SoundSphere_C|SetNearbySpheres%20 _asbp_sound_sphere (Utilities|Array|MakeArray 0)))
              (:CastFailed
                _))))
        (Transformation|SetWorldScale3D (Variables|/Game/ItemBP/BP_SoundCube.BP_SoundCube_C|GetCube (Utilities|Array|Get(acopy) SoundCube _array_index)) (Math|Vector|MakeVector (* _array_element (Variables|Default|GetScaleFact)) 0.25 0.0))))))