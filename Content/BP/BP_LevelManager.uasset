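; BP_LevelManager is a trigger-box actor, apparently an unfinished switcher for a NiagaraID selection shown by BP_CPPVisualizer.
; BeginPlay enables input and caches the visualizer; box overlaps track whether BP_Player is inside.
; Increment and decrement inputs check that flag but trigger nothing.
; ChangeMode resets and respawns the visualizer; Decrement lowers NiagaraID to zero at minimum, while Increment and UpdateName are empty.
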(event OnComponentBeginOverlap(Box)
  (params (OverlappedComponent :type Primitive%20Component%20Object%20Reference) (OtherActor :type Actor%20Object%20Reference) (OtherComp :type Primitive%20Component%20Object%20Reference) (OtherBodyIndex :type Integer) (bFromSweep :type Boolean) (SweepResult :type Hit%20Result%20Structure%20%28by%20ref%29))
  (Utilities|Casting|CastToBP_Player OtherActor)
  (Variables|Default|SetPlayerIsIn true))

(event OnComponentEndOverlap(Box)
  (params (OverlappedComponent :type Primitive%20Component%20Object%20Reference) (OtherActor :type Actor%20Object%20Reference) (OtherComp :type Primitive%20Component%20Object%20Reference) (OtherBodyIndex :type Integer))
  (Utilities|Casting|CastToBP_Player OtherActor)
  (Variables|Default|SetPlayerIsIn false))

(event Input|EnhancedActionEvents|EnhancedInputActionIA_Decrement
  (params (ActionValue :type Boolean) (ElapsedSeconds :type Float%20%28double-precision%29) (TriggeredSeconds :type Float%20%28double-precision%29) (InputAction :type Input%20Action%20Object%20Reference :default "/Game/Player/inputs/Actions/IA_Decrement.IA_Decrement"))
  (:Completed
    (if (Variables|Default|GetPlayerIsIn)
      _)))

(event Input|EnhancedActionEvents|EnhancedInputActionIA_Increment
  (params (ActionValue :type Boolean) (ElapsedSeconds :type Float%20%28double-precision%29) (TriggeredSeconds :type Float%20%28double-precision%29) (InputAction :type Input%20Action%20Object%20Reference :default "/Game/Player/inputs/Actions/IA_Increment.IA_Increment"))
  (:Completed
    (if (Variables|Default|GetPlayerIsIn)
      _)))

(event EventBeginPlay
  (Input|EnableInput (Game|GetPlayerController 0))
  (bind _returnvalue (Actor|GetActorOfClass "/Game/BP/BP_CPPVisualizer.BP_CPPVisualizer_C"))
  (Variables|Default|SetCPPVisaulizer _returnvalue))

(event Collision|EventActorBeginOverlap
  (params (OtherActor :type Actor%20Object%20Reference)))

(event EventTick
  (params (DeltaSeconds :type Float%20%28single-precision%29)))

(fn ConstructionScript)

(fn Decrement
  (if (> (Variables|Default|GetNiagaraID) 0)
    (Variables|Default|SetNiagaraID (- (Variables|Default|GetNiagaraID) 1))
    (CallFunction|UpdateName)))

(fn Increment)

(fn UpdateName)