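; BP_VFXManager is an in-world selector that lets the player preview Niagara projectile effects while standing in its box.
; Increment and decrement inputs step a clamped index through the template array, updating the text label and Niagara component.
; BeginPlay restores the index from the "SelectedSkin" save, but creates missing saves under "SaveSlot".
; SavePreference writes the choice back, though nothing here calls it.
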(event OnComponentBeginOverlap(Box)
  (params (OverlappedComponent :type Primitive%20Component%20Object%20Reference) (OtherActor :type Actor%20Object%20Reference) (OtherComp :type Primitive%20Component%20Object%20Reference) (OtherBodyIndex :type Integer) (bFromSweep :type Boolean) (SweepResult :type Hit%20Result%20Structure%20%28by%20ref%29))
  (Utilities|Casting|CastToBP_Player OtherActor)
  (Variables|Default|SetPlayerIsIn true))

(event OnComponentEndOverlap(Box)
  (params (OverlappedComponent :type Primitive%20Component%20Object%20Reference) (OtherActor :type Actor%20Object%20Reference) (OtherComp :type Primitive%20Component%20Object%20Reference) (OtherBodyIndex :type Integer))
  (Utilities|Casting|CastToBP_Player OtherActor)
  (Variables|Default|SetPlayerIsIn false))

(event Input|EnhancedActionEvents|EnhancedInputActionIA_Decrement
  (params (ActionValue :type Boolean) (ElapsedSeconds :type Float%20%28double-precision%29) (TriggeredSeconds :type Float%20%28double-precision%29) (InputAction :type Input%20Action%20Object%20Reference :default "/Game/Player/inputs/Actions/IA_Decrement.IA_Decrement"))
  (:Completed
    (if (Variables|Default|GetPlayerIsIn)
      (CallFunction|Decrement))))

(event Input|EnhancedActionEvents|EnhancedInputActionIA_Increment
  (params (ActionValue :type Boolean) (ElapsedSeconds :type Float%20%28double-precision%29) (TriggeredSeconds :type Float%20%28double-precision%29) (InputAction :type Input%20Action%20Object%20Reference :default "/Game/Player/inputs/Actions/IA_Increment.IA_Increment"))
  (:Completed
    (if (Variables|Default|GetPlayerIsIn)
      (CallFunction|Increment))))

(event EventBeginPlay
  (Input|EnableInput (Game|GetPlayerController 0))
  (bind _returnvalue (SaveGame|DoesSaveGameExist "SelectedSkin"))
  (if _returnvalue
    (bind _returnvalue_2 (SaveGame|LoadGamefromSlot "SelectedSkin"))
    (bind _asbp_skin_selection (Utilities|Casting|CastToBP_SkinSelection _returnvalue_2)
      (:then
        (Variables|Default|SetNiagaraID (Variables|/Game/BP/Data/BP_SkinSelection.BP_SkinSelection_C|GetProjectile _asbp_skin_selection))
        (Development|PrintString "load")
        (CallFunction|UpdateName :!label _label))
      (:CastFailed
        (Development|PrintString "cast de save failed")))
    (else
      (bind _returnvalue_3 (SaveGame|CreateSaveGameObject "/Game/BP/Data/BP_SkinSelection.BP_SkinSelection_C"))
      (SaveGame|SaveGametoSlot _returnvalue_3 "SaveSlot")
      (Development|PrintString "create")
      (goto _label))))

(event Collision|EventActorBeginOverlap
  (params (OtherActor :type Actor%20Object%20Reference)))

(event EventTick
  (params (DeltaSeconds :type Float%20%28single-precision%29)))

(fn ConstructionScript)

(fn Decrement
  (if (> (Variables|Default|GetNiagaraID) 0)
    (Variables|Default|SetNiagaraID (- (Variables|Default|GetNiagaraID) 1))
    (CallFunction|UpdateName)))

(fn Increment
  (if (< (Variables|Default|GetNiagaraID) (- (Utilities|Array|Length (Variables|Default|GetNiagaraTemplate)) 1))
    (Variables|Default|SetNiagaraID (+ (Variables|Default|GetNiagaraID) 1))
    (CallFunction|UpdateName)))

(fn UpdateName
  (Rendering|Components|TextRender|SetText (Variables|Default|GetTextRender) (Utilities|Text|FormatText "VFX Selected :  
{prout}" (Utilities|GetObjectName (Utilities|Array|Get(acopy) (Variables|Default|GetNiagaraTemplate) (Variables|Default|GetNiagaraID)))))
  (Class|NiagaraComponent|SetAsset (Variables|Default|GetNiagara) (Utilities|Array|Get(acopy) (Variables|Default|GetNiagaraTemplate) (Variables|Default|GetNiagaraID)) true))

(fn SavePreference
  (bind _returnvalue (SaveGame|LoadGamefromSlot "SelectedSkin"))
  (bind _asbp_skin_selection (Utilities|Casting|CastToBP_SkinSelection _returnvalue))
  (Variables|/Game/BP/Data/BP_SkinSelection.BP_SkinSelection_C|SetProjectile _asbp_skin_selection (Variables|Default|GetNiagaraID))
  (SaveGame|SaveGametoSlot _returnvalue "SelectedSkin")
  (Development|PrintString "SAved")
  (Audio|PlaySound2D "/Game/AudioFile/VFX/Data_Point_01.Data_Point_01" 1.0 1.0 0.0 0 0))