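; Object pool manager that pre-spawns a configurable number of ObjectClass actors on BeginPlay, hidden and tagged "Inactive".
; GetPooledObject reuses the first inactive actor, moving it to the requested location and rotation, resetting scale to one, replacing its tags and unhiding it.
; When none are free, it spawns a new actor and adds it to the pool.
; Availability relies solely on the tag; this Blueprint has no return-to-pool function.
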(event EventBeginPlay
  (Utilities|FlowControl|DoOnce false
    (:Completed
      (for _index (range 0 (Variables|Default|GetPoolSize))
        (bind _returnvalue (Game|SpawnActorfromClass (Variables|Default|GetObjectClass) (Math|Transform|MakeTransform "0, 0, 0") "AdjustIfPossibleButAlwaysSpawn" "MultiplyWithRoot" 0 0))
        (Variables|/Script/Engine.Actor|SetTags _returnvalue (Utilities|Array|MakeArray "Inactive"))
        (Rendering|SetActorHiddenInGame _returnvalue true)
        (Utilities|Array|Add (Variables|Default|GetPooledObjects) _returnvalue)))))

(event Collision|EventActorBeginOverlap
  (params (OtherActor :type Actor%20Object%20Reference)))

(event EventTick
  (params (DeltaSeconds :type Float%20%28single-precision%29)))

(fn ConstructionScript)

(fn GetPooledObject
  (params (SpawnTransform :type Transform))
  (bind (_location _rotation) (Math|Transform|BreakTransform SpawnTransform))
  (for _array_element (Variables|Default|GetPooledObjects)
    (if (Actor|ActorHasTag _array_element "Inactive")
      (Transformation|SetActorLocation _array_element _location false true)
      (Transformation|SetActorRotation _array_element _rotation)
      (Transformation|SetActorScale3D _array_element "1.000000,1.000000,1.000000")
      (Variables|/Script/Engine.Actor|SetTags _array_element (Utilities|Array|MakeArray "None"))
      (Rendering|SetActorHiddenInGame _array_element false)
      (return _array_element)))
  (bind _returnvalue (Game|SpawnActorfromClass (Variables|Default|GetObjectClass) SpawnTransform "Undefined" "MultiplyWithRoot" 0 0))
  (Rendering|SetActorHiddenInGame _returnvalue false)
  (Utilities|Array|Add (Variables|Default|GetPooledObjects) _returnvalue)
  (return _returnvalue))