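; BP_Projectile is a projectile that ignores hits on the player-type spaceship BP_NewSpaceShip and takes its visuals from BP_VFXManager.
; On BeginPlay it sets its Niagara trail by the manager's NiagaraID, which also selects the impact effect.
; Impacts tag it Inactive and expire it shortly after, while passing an X limit tags it Inactive and stops it.
; ReactivateSpeed restores speed limits, but its velocity call is unwired; the boss cast leads nowhere.
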(event OnComponentHit(Box)
  (params (HitComponent :type Primitive%20Component%20Object%20Reference) (OtherActor :type Actor%20Object%20Reference) (OtherComp :type Primitive%20Component%20Object%20Reference) (NormalImpulse :type Vector :default "0, 0, 0") (Hit :type Hit%20Result%20Structure%20%28by%20ref%29))
  (bind _location (Collision|BreakHitResult Hit))
  (bind (_x _y _z) (Math|Vector|BreakVector _location))
  (Utilities|Casting|CastToBP_NewSpaceShip OtherActor
    (:CastFailed
      (Niagara|SpawnSystematLocation (Utilities|Array|Get(acopy) (Variables|/Game/BP/BP_VFXManager.BP_VFXManager_C|GetHits (stale EventBeginPlay _returnvalue)) (Math|Integer|Clamp(Integer) (Variables|/Game/BP/BP_VFXManager.BP_VFXManager_C|GetNiagaraID (stale EventBeginPlay _returnvalue)) 0 20)) (Math|Vector|MakeVector (- _x 18.0) _y _z))
      (Variables|/Script/Engine.Actor|SetTags self (Utilities|Array|MakeArray "Inactive"))
      (Actor|SetLifeSpan 0.3)
      (Utilities|Casting|CastToBP_Boss OtherActor))))

(event EventBeginPlay
  (bind _returnvalue (Actor|GetActorOfClass "/Game/BP/BP_VFXManager.BP_VFXManager_C"))
  (Class|NiagaraComponent|SetAsset (Variables|Default|GetNiagara) (Utilities|Array|Get(acopy) (Variables|/Game/BP/BP_VFXManager.BP_VFXManager_C|GetNiagaraTemplate _returnvalue) (Math|Integer|Clamp(Integer) (Variables|/Game/BP/BP_VFXManager.BP_VFXManager_C|GetNiagaraID _returnvalue) 0 20)) true))

(event EventTick
  (params (DeltaSeconds :type Float%20%28single-precision%29))
  (if (> (.x (Transformation|GetActorLocation)) 5e+03)
    (Variables|/Script/Engine.Actor|SetTags self (Utilities|Array|MakeArray "Inactive"))
    (Game|Components|ProjectileMovement|SetVelocityinLocalSpace (Variables|Default|GetProjectileMovement) "0, 0, 0")))

(fn ConstructionScript)

(fn ReactivateSpeed
  (params (NewParam :type Vector))
  (bind _projectilemovement (Variables|Default|GetProjectileMovement))
  (Variables|/Script/Engine.ProjectileMovementComponent|SetMaxSpeed _projectilemovement 3.5e+03)
  (Variables|/Script/Engine.ProjectileMovementComponent|SetInitialSpeed _projectilemovement 3.5e+03))