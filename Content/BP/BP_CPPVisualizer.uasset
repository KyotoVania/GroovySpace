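; Blueprint music visualizer actor that plays a track and keeps its visuals in step with audio playback.
; Playback percent updates from the AudioComponent are scaled by MusicDuration in SynthesiaScale and passed as a time to UpdateVisualizerAtTime.
; StartLevel starts the audio.
; IA_PauseAction or Unpausepause toggles it: pausing also pauses the game and opens WBP_PauseOptionMenu, while resuming here only unpauses the audio.
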(event Custom|OnPlaybackChange
  (params (PlayingSoundWave :type Sound%20Wave%20Object%20Reference) (PlaybackPercent :type Float%20%28single-precision%29))
  ;[0.15 0.15 0.15 0.5] SetPlayBackLink
  (if (not (Variables|Default|GetPaused))
    (if (Audio|Components|Audio|IsPlaying (Variables|Default|GetAudioComponent))
      (CallFunction|SynthesiaScale (Variables|Default|GetMusicDuration) PlaybackPercent))))

(event Custom|StartLevel
  ;[0.15 0.15 0.15 0.5] Pause/Start
  (Development|PrintString "Hello starting play in bp")
  (Audio|Components|Audio|Play (Variables|Default|GetAudioComponent) 0.0))

(event Custom|Unpause%20pause
  (bind _audiocomponent (Variables|Default|GetAudioComponent))
  ;[0.15 0.15 0.15 0.5] Pause/Start
  (if (Variables|Default|GetPaused)
    (Class|AudioComponent|SetPaused _audiocomponent false)
    (Variables|Default|SetPaused false)
    (else
      (Class|AudioComponent|SetPaused _audiocomponent true)
      (Game|SetGamePaused true)
      (bind _returnvalue (UserInterface|CreateWidget "/Game/HUD/WBP_PauseOptionMenu.WBP_PauseOptionMenu_C" (Game|GetPlayerController 0)))
      (UserInterface|Viewport|AddtoViewport _returnvalue -1)
      (Variables|Default|SetPaused true))))

(event Input|EnhancedActionEvents|EnhancedInputActionIA_PauseAction
  (params (ActionValue :type Boolean) (ElapsedSeconds :type Float%20%28double-precision%29) (TriggeredSeconds :type Float%20%28double-precision%29) (InputAction :type Input%20Action%20Object%20Reference :default "/Game/Player/inputs/Actions/IA_PauseAction.IA_PauseAction"))
  (bind _audiocomponent (Variables|Default|GetAudioComponent))
  ;[0.15 0.15 0.15 0.5] Pause/Start
  (:Completed
    (if (Variables|Default|GetPaused)
      (Class|AudioComponent|SetPaused _audiocomponent false)
      (Variables|Default|SetPaused false)
      (else
        (Class|AudioComponent|SetPaused _audiocomponent true)
        (Game|SetGamePaused true)
        (bind _returnvalue (UserInterface|CreateWidget "/Game/HUD/WBP_PauseOptionMenu.WBP_PauseOptionMenu_C" (Game|GetPlayerController 0)))
        (UserInterface|Viewport|AddtoViewport _returnvalue -1)
        (Variables|Default|SetPaused true)))))

(event EventBeginPlay
  (Utilities|FlowControl|Sequence
    (:then_2
      ;[0.15 0.15 0.15 0.5] SetPlayBackLink
      (EventDispatchers|BindEventtoOnAudioPlaybackPercent (Variables|Default|GetAudioComponent) (delegate Custom|OnPlaybackChange))
      (Development|PrintString "binding to sounbd"))))

(event Collision|EventActorBeginOverlap
  (params (OtherActor :type Actor%20Object%20Reference)))

(fn ConstructionScript)

(fn SynthesiaScale
  (params (MusicDuration :type Float%20%28double-precision%29) (PercentagePlayed :type Float%20%28double-precision%29) (SoundCube :type Array%20of%20BP%20Sound%20Cube%20Object%20References))
  (Utilities|FlowControl|Sequence
    (:then_0
      ;[0.15 0.15 0.15 0.5] Get Space In track
      (bind _output_get (Variables|Default|SetSpace%20in%20Music (* MusicDuration PercentagePlayed)))
      (Class|VisualizerActor|UpdateVisualizeratTime _output_get))))