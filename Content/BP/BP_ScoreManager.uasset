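; BP_ScoreManager is an Actor Blueprint that, despite its score-manager name, only handles health regeneration.
; Each Tick, while IsRegeningHealth is set, it raises CurrentHealth by HealthRegenRate scaled by world delta seconds, clamped between zero and MaxHealth.
; A check for full health is never executed, and nothing in the graph changes the regeneration flag.
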(event EventBeginPlay)

(event Collision|EventActorBeginOverlap
  (params (OtherActor :type Actor%20Object%20Reference)))

(event EventTick
  (params (DeltaSeconds :type Float%20%28single-precision%29))
  (if (Variables|Default|GetIsRegeningHealth?)
    (Variables|Default|SetCurrentHealth (Math|Float|Clamp(Float) (+ (Variables|Default|GetCurrentHealth) (* (Utilities|Time|GetWorldDeltaSeconds) (Variables|Default|GetHealthRegenRate))) 0.0 (Variables|Default|GetMaxHealth)))))

(fn ConstructionScript)