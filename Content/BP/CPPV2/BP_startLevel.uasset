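; Trigger actor that sends the player to the ScifiCityscape_Showcase level when the spaceship character overlaps it.
; On the first overlap only, it sets the display background and a random movie index, likely for the loading screen.
; It then plays the LS_flyingout level sequence, waits for a delay derived from its end time, and opens the level.
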(event EventBeginPlay)

(event Collision|EventActorBeginOverlap
  (params (OtherActor :type Actor%20Object%20Reference))
  (bind _asspaceship_character (Utilities|Casting|CastToSpaceshipCharacter OtherActor))
  (Utilities|IsValid _asspaceship_character
    (:Is%20Valid
      (Utilities|FlowControl|DoOnce false
        (:Completed
          (Class|AsyncLoadingScreenLibrary|SetDisplayBackgroundIndex 3)
          (Class|AsyncLoadingScreenLibrary|SetDisplayMovieIndex (Math|Random|RandomInteger 3))
          (bind _returnvalue (Sequencer|Player|CreateLevelSequencePlayer "/Game/lobby_sequence/LS_flyingout.LS_flyingout"))
          (Sequencer|Player|Play _returnvalue :!class /Script/MovieScene.MovieSceneSequencePlayer)
          (Utilities|FlowControl|Delay (Class|TimeManagementBlueprintLibrary|ToSeconds(QualifiedFrameTime) (Class|MovieSceneSequencePlayer|GetEndTime _returnvalue)))
          (Game|OpenLevel(byName) "ScifiCityscape_Showcase"))))))

(event EventTick
  (params (DeltaSeconds :type Float%20%28single-precision%29)))

(fn ConstructionScript)