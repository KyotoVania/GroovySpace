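; BP_SkinManager lets a skin be chosen by stepping an index, misleadingly named NiagaraID, through a template array without wrapping.
; Each step applies that skin's white and black materials to two StarSparrow preview meshes.
; It then pushes them to the BP_NewSpaceShip found in the level and, only if that exists, sets matching sphere materials on BP_CPPVisualizer.
; SavePreference is an empty, uncalled stub, and the selection label update is disconnected.
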(fn ConstructionScript)

(fn Decrement
  (if (> (Variables|Default|GetNiagaraID) 0)
    (Variables|Default|SetNiagaraID (- (Variables|Default|GetNiagaraID) 1))
    (CallFunction|UpdateName)
    (CallFunction|UpdateSkinPlayer)))

(fn Increment
  (if (< (Variables|Default|GetNiagaraID) (- (Utilities|Array|Length (Variables|Default|GetSkinTemplatre_0)) 1))
    (Variables|Default|SetNiagaraID (+ (Variables|Default|GetNiagaraID) 1))
    (CallFunction|UpdateName)
    (CallFunction|UpdateSkinPlayer)))

(fn UpdateName
  (CallFunction|UpdateSkin))

(fn UpdateSkin
  (bind _niagaraid (Variables|Default|GetNiagaraID))
  (bind _skintemplatre_0 (Variables|Default|GetSkinTemplatre_0))
  (bind _output (Utilities|Array|Get(acopy) _skintemplatre_0 _niagaraid))
  (bind (_whitematerial _blackmaterial) (Utilities|Struct|BreakMaterialSet _output))
  (Rendering|Material|SetMaterial (Variables|Default|GetStarSparrow01) 0 _whitematerial)
  (Rendering|Material|SetMaterial (Variables|Default|GetStarSparrow02) 0 _blackmaterial))

(fn SavePreference)

(fn UpdateSkinPlayer
  (bind _skintemplatre_0 (Variables|Default|GetSkinTemplatre_0))
  (bind _niagaraid (Variables|Default|GetNiagaraID))
  (bind _output (Utilities|Array|Get(acopy) _skintemplatre_0 _niagaraid))
  (bind (_whitematerial _blackmaterial) (Utilities|Struct|BreakMaterialSet _output))
  (bind _returnvalue (Actor|GetActorOfClass "/Game/BP/BP_NewSpaceShip.BP_NewSpaceShip_C"))
  (Utilities|IsValid _returnvalue
    (:Is%20Valid
      (Variables|/Game/BP/BP_NewSpaceShip.BP_NewSpaceShip_C|SetMaterialTabl _returnvalue (Utilities|Array|MakeArray _whitematerial _blackmaterial))
      (Default|ApplyText _returnvalue)
      (Development|PrintString "we cahnge the shit for ")
      (bind _returnvalue_2 (Actor|GetActorOfClass "/Game/BP/BP_CPPVisualizer.BP_CPPVisualizer_C"))
      (Utilities|IsValid _returnvalue_2
        (:Is%20Valid
          (Variables|/Script/Spaceship.VisualizerActor|SetColorMaterials _returnvalue_2 (Utilities|Array|Get(acopy) (Variables|Default|GetSkinSphereTemplatre) (Variables|Default|GetNiagaraID))))))))