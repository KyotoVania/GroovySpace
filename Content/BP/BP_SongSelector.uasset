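; BP_SongSelector is an in-world pre-game console for picking the song, difficulty and track shape, then launching the level.
; Input actions work while the player is inside InteractBox, updating text displays and writing each change to the SelectedSkin save slot.
; When the spaceship enters StarterBox, it saves those choices plus skin and VFX from their managers, plays a fly-out sequence and opens the cityscape level.
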(event OnComponentBeginOverlap(StarterBox)
  (params (OverlappedComponent :type Primitive%20Component%20Object%20Reference) (OtherActor :type Actor%20Object%20Reference) (OtherComp :type Primitive%20Component%20Object%20Reference) (OtherBodyIndex :type Integer) (bFromSweep :type Boolean) (SweepResult :type Hit%20Result%20Structure%20%28by%20ref%29))
  (Utilities|Casting|CastToBP_NewSpaceShip OtherActor)
  (Utilities|FlowControl|DoOnce false
    (:Completed
      (CallFunction|SaveEverythings)
      (Class|AsyncLoadingScreenLibrary|SetDisplayBackgroundIndex 3)
      (Class|AsyncLoadingScreenLibrary|SetDisplayMovieIndex (Math|Random|RandomInteger 3))
      (bind _returnvalue (Sequencer|Player|CreateLevelSequencePlayer "/Game/lobby_sequence/LS_flyingout.LS_flyingout"))
      (Sequencer|Player|Play _returnvalue :!class /Script/MovieScene.MovieSceneSequencePlayer)
      (Utilities|FlowControl|Delay (Class|TimeManagementBlueprintLibrary|ToSeconds(QualifiedFrameTime) (Class|MovieSceneSequencePlayer|GetEndTime _returnvalue)))
      (Game|OpenLevel(byName) "ScifiCityscape_Showcase"))))

(event OnComponentBeginOverlap(InteractBox)
  (params (OverlappedComponent :type Primitive%20Component%20Object%20Reference) (OtherActor :type Actor%20Object%20Reference) (OtherComp :type Primitive%20Component%20Object%20Reference) (OtherBodyIndex :type Integer) (bFromSweep :type Boolean) (SweepResult :type Hit%20Result%20Structure%20%28by%20ref%29))
  (Utilities|Casting|CastToBP_Player OtherActor)
  (Variables|Default|SetPlayerIsIn true))

(event OnComponentEndOverlap(InteractBox)
  (params (OverlappedComponent :type Primitive%20Component%20Object%20Reference) (OtherActor :type Actor%20Object%20Reference) (OtherComp :type Primitive%20Component%20Object%20Reference) (OtherBodyIndex :type Integer))
  (Utilities|Casting|CastToBP_Player OtherActor)
  (Variables|Default|SetPlayerIsIn false))

(event Input|EnhancedActionEvents|EnhancedInputActionIA_IncDifficulty
  (params (ActionValue :type Boolean) (ElapsedSeconds :type Float%20%28double-precision%29) (TriggeredSeconds :type Float%20%28double-precision%29) (InputAction :type Input%20Action%20Object%20Reference :default "/Game/Player/inputs/Actions/IA_IncDifficulty.IA_IncDifficulty"))
  (:Completed
    (if (Variables|Default|GetPlayerIsIn)
      (CallFunction|IncrementDiff -1))))

(event Input|EnhancedActionEvents|EnhancedInputActionIA_DecDifficulty
  (params (ActionValue :type Boolean) (ElapsedSeconds :type Float%20%28double-precision%29) (TriggeredSeconds :type Float%20%28double-precision%29) (InputAction :type Input%20Action%20Object%20Reference :default "/Game/Player/inputs/Actions/IA_DecDifficulty.IA_DecDifficulty"))
  (:Completed
    (if (Variables|Default|GetPlayerIsIn)
      (CallFunction|IncrementDiff 1))))

(event Input|EnhancedActionEvents|EnhancedInputActionIA_Decrement
  (params (ActionValue :type Boolean) (ElapsedSeconds :type Float%20%28double-precision%29) (TriggeredSeconds :type Float%20%28double-precision%29) (InputAction :type Input%20Action%20Object%20Reference :default "/Game/Player/inputs/Actions/IA_Decrement.IA_Decrement"))
  (:Completed
    (if (Variables|Default|GetPlayerIsIn)
      (CallFunction|Decrement))))

(event Input|EnhancedActionEvents|EnhancedInputActionIA_Increment
  (params (ActionValue :type Boolean) (ElapsedSeconds :type Float%20%28double-precision%29) (TriggeredSeconds :type Float%20%28double-precision%29) (InputAction :type Input%20Action%20Object%20Reference :default "/Game/Player/inputs/Actions/IA_Increment.IA_Increment"))
  (:Completed
    (if (Variables|Default|GetPlayerIsIn)
      (CallFunction|Increment))))

(event Input|EnhancedActionEvents|EnhancedInputActionIA_SwitchShape
  (params (ActionValue :type Boolean) (ElapsedSeconds :type Float%20%28double-precision%29) (TriggeredSeconds :type Float%20%28double-precision%29) (InputAction :type Input%20Action%20Object%20Reference :default "/Game/Player/inputs/Actions/IA_SwitchShape.IA_SwitchShape"))
  (:Completed
    (if (Variables|Default|GetPlayerIsIn)
      (CallFunction|SwitchShape))))

(event EventBeginPlay
  (Input|EnableInput (Game|GetPlayerController 0))
  (bind _returnvalue (SaveGame|DoesSaveGameExist "SelectedSkin"))
  (if _returnvalue
    (bind _returnvalue_2 (SaveGame|LoadGamefromSlot "SelectedSkin"))
    (bind _asbp_skin_selection (Utilities|Casting|CastToBP_SkinSelection _returnvalue_2))
    (Variables|Default|SetAs%20BP%20Skin%20Selection _asbp_skin_selection)
    (Variables|Default|SetcurrentIndex_Difficulty (Variables|/Game/BP/Data/BP_SkinSelection.BP_SkinSelection_C|GetDiff _asbp_skin_selection))
    (else
      (Development|PrintString "We create saave")
      (bind _returnvalue_3 (SaveGame|CreateSaveGameObject "/Game/BP/Data/BP_SkinSelection.BP_SkinSelection_C"))
      (Variables|Default|SetAs%20BP%20Skin%20Selection _returnvalue_3)
      (Variables|/Game/BP/Data/BP_SkinSelection.BP_SkinSelection_C|SetDiff _returnvalue_3 1)
      (SaveGame|SaveGametoSlot _returnvalue_3 "SelectedSkin")
      (CallFunction|UpdateDiff)
      (CallFunction|UpdateName)
      (Rendering|Components|TextRender|SetText (Variables|Default|Getshape) (|GenerictoText (Variables|/Game/BP/Data/BP_SkinSelection.BP_SkinSelection_C|GetShape (Variables|Default|GetAs%20BP%20Skin%20Selection)))))))

(event Collision|EventActorBeginOverlap
  (params (OtherActor :type Actor%20Object%20Reference)))

(event EventTick
  (params (DeltaSeconds :type Float%20%28single-precision%29)))

(fn ConstructionScript)

(fn Decrement
  (if (> (Variables|Default|GetcurrentIndex) 0)
    (bind _output_get (Variables|Default|SetcurrentIndex (- (Variables|Default|GetcurrentIndex) 1)))
    (Variables|Default|SetselectedSound (Utilities|Array|Get(acopy) (Variables|Default|GetsoundList) _output_get))
    (CallFunction|UpdateName)
    (Audio|PlaySound2D "/Game/AudioFile/VFX/Confirm_03DEC.Confirm_03DEC" 1.0 1.0 0.0 0 0)))

(fn Increment
  (if (< (Variables|Default|GetcurrentIndex) (- (Utilities|Array|Length (Variables|Default|GetsoundList)) 1))
    (bind _output_get (Variables|Default|SetcurrentIndex (+ (Variables|Default|GetcurrentIndex) 1)))
    (Variables|Default|SetselectedSound (Utilities|Array|Get(acopy) (Variables|Default|GetsoundList) _output_get))
    (CallFunction|UpdateName)
    (Audio|PlaySound2D "/Game/AudioFile/VFX/Confirm_02Inc.Confirm_02Inc" 1.0 1.0 0.0 0 0)))

(fn SetSound
  (bind _as_bp_skin_selection (Variables|Default|GetAs%20BP%20Skin%20Selection))
  (Variables|/Game/BP/Data/BP_SkinSelection.BP_SkinSelection_C|SetLastSong _as_bp_skin_selection (Variables|Default|GetselectedSound))
  (SaveGame|SaveGametoSlot _as_bp_skin_selection "SelectedSkin"))

(fn UpdateName
  (Rendering|Components|TextRender|SetText (Variables|Default|GetTextRender) (Utilities|Text|FormatText "Song Selected :  
{prout}" (Utilities|GetObjectName (Variables|Default|GetselectedSound))))
  (CallFunction|SetSound))

(fn IncrementDiff
  (params (input :type Integer))
  (if (and (<= (+ (Variables|Default|GetcurrentIndex_Difficulty) input) 10) (> (+ (Variables|Default|GetcurrentIndex_Difficulty) input) 0))
    (Variables|Default|SetcurrentIndex_Difficulty (+ input (Variables|Default|GetcurrentIndex_Difficulty)))
    (CallFunction|UpdateDiff)
    (Audio|PlaySound2D "/Game/AudioFile/VFX/Confirm_06.Confirm_06" 1.0 1.0 0.0 0 0)))

(fn UpdateDiff
  (bind _currentindex_difficulty (Variables|Default|GetcurrentIndex_Difficulty))
  (bind _as_bp_skin_selection (Variables|Default|GetAs%20BP%20Skin%20Selection))
  (Rendering|Components|TextRender|SetText (Variables|Default|GetdiffText) (Utilities|Text|ToText(Integer) _currentindex_difficulty))
  (Variables|/Game/BP/Data/BP_SkinSelection.BP_SkinSelection_C|SetDiff _as_bp_skin_selection _currentindex_difficulty)
  (SaveGame|SaveGametoSlot _as_bp_skin_selection "SelectedSkin"))

(fn SwitchShape
  (bind _as_bp_skin_selection (Variables|Default|GetAs%20BP%20Skin%20Selection))
  (Utilities|IsValid _as_bp_skin_selection
    (:Is%20Valid
      (if (Utilities|Enum|Equal(Enum) (Variables|/Game/BP/Data/BP_SkinSelection.BP_SkinSelection_C|GetShape _as_bp_skin_selection) "Circle")
        (Variables|/Game/BP/Data/BP_SkinSelection.BP_SkinSelection_C|SetShape _as_bp_skin_selection "HalfCircle")
        (else
          (Variables|/Game/BP/Data/BP_SkinSelection.BP_SkinSelection_C|SetShape _as_bp_skin_selection "Circle")))
      (SaveGame|SaveGametoSlot _as_bp_skin_selection "SelectedSkin")
      (Rendering|Components|TextRender|SetText (Variables|Default|Getshape) (|GenerictoText (Variables|/Game/BP/Data/BP_SkinSelection.BP_SkinSelection_C|GetShape _as_bp_skin_selection)))
      (Audio|PlaySound2D "/Game/AudioFile/VFX/Confirm_07.Confirm_07" 1.0 1.0 0.0 0 0))))

(fn SaveEverythings
  (bind _selectedsound (Variables|Default|GetselectedSound))
  (bind _as_bp_skin_selection (Variables|Default|GetAs%20BP%20Skin%20Selection))
  (bind _returnvalue (Actor|GetActorOfClass "/Game/BP/BP_SkinManager.BP_SkinManager_C"))
  (Development|PrintText (Utilities|Text|FormatText "last save gve skin : {vé}" (Variables|/Game/BP/BP_SkinManager.BP_SkinManager_C|GetNiagaraID _returnvalue)))
  (bind _returnvalue_2 (Actor|GetActorOfClass "/Game/BP/BP_VFXManager.BP_VFXManager_C"))
  (Development|PrintText (Utilities|Text|FormatText "last save gve VFX : {vé}" (Variables|/Game/BP/BP_VFXManager.BP_VFXManager_C|GetNiagaraID _returnvalue_2)))
  (Variables|/Game/BP/Data/BP_SkinSelection.BP_SkinSelection_C|SetProjectile _as_bp_skin_selection (Variables|/Game/BP/BP_VFXManager.BP_VFXManager_C|GetNiagaraID _returnvalue_2))
  (Variables|/Game/BP/Data/BP_SkinSelection.BP_SkinSelection_C|SetSkin _as_bp_skin_selection (Variables|/Game/BP/BP_SkinManager.BP_SkinManager_C|GetNiagaraID _returnvalue))
  (Variables|/Game/BP/Data/BP_SkinSelection.BP_SkinSelection_C|SetLastSong _as_bp_skin_selection _selectedsound)
  (Development|PrintText (Utilities|Text|FormatText "last save gve VFX : {vé}" _selectedsound))
  (Variables|/Game/BP/Data/BP_SkinSelection.BP_SkinSelection_C|SetFirstTime? _as_bp_skin_selection false)
  (SaveGame|SaveGametoSlot _as_bp_skin_selection "SelectedSkin"))